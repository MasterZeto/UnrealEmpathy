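; Interactive whiteboard actor that lets the player draw with the mouse, with F toggling the view between board and pawn.
; While in use, Tick traces from the cursor and holding left mouse spawns PenColour decals at the hit location, alongside a pen-press timeline.
; The pen mesh follows the deprojected cursor through a scaled offset from the board.
; Fixed decal rotation and pen depth tie it to one world orientation and position.
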(event EventTick
  (params (DeltaSeconds :type Float%20%28single-precision%29))
  (bind _returnvalue (Game|GetPlayerController 0))
  (bind _returnvalue_2 (Game|GetPlayerController 0))
  (bind _mainpen (Variables|Default|GetMainPen))
  (bind _whiteboard (Variables|Default|Getwhiteboard))
  (bind _worldlocation (Game|Player|ConvertMouseLocationToWorldSpace _returnvalue_2))
  (bind (_worldlocation_2 _worlddirection) (Game|Player|ConvertMouseLocationToWorldSpace _returnvalue))
  (bind _returnvalue_3 (Transformation|GetWorldLocation _whiteboard))
  (bind _returnvalue_4 (- _worldlocation _returnvalue_3))
  (bind _returnvalue_5 (* _returnvalue_4 "5.000000,0.000000,5.000000"))
  (bind _returnvalue_6 (+ _returnvalue_5 _returnvalue_3))
  (bind (_x _y _z) (Math|Vector|BreakVector _returnvalue_6))
  ;[1 1 1] Event Tick
  (Utilities|FlowControl|Sequence
    (:then_0
      ;[1 1 1] Line Trace From Mouse Pointer
      (bind _outhit (Collision|LineTraceByChannel _worldlocation_2 (+ _worldlocation_2 (* _worlddirection 1e+03)) "TraceTypeQuery2" false (Utilities|Array|MakeArray (Game|GetPlayerCharacter 0)) "None"))
      ;[1 1 1] Spawn Decal And Animate Pen Pressing
      (if (and (Variables|Default|GetUsingWhiteBoard) (Variables|Default|Getlmbheld))
        (Development|PrintString "Pressed")
        (Rendering|Decal|SpawnDecalatLocation (Variables|Default|GetPenColour) "2.000000,2.000000,2.000000" (.Location (Collision|BreakHitResult _outhit)) "0.000000,90.000000,90.000000" 0.0) ; Rotation May Need Updating If Rotating Blueprint
        (bind _newtrack_0 (Timeline|PushPenToBoard Play)
          (:Update
            (Transformation|SetRelativeLocation _mainpen (+ _newtrack_0 (Variables|/Script/Engine.SceneComponent|GetRelativeLocation _mainpen)) false false)))))
    (:then_1
      ;[1 1 1] Update Pen Location To Mouse Pointer
      (if (Variables|Default|GetUsingWhiteBoard)
        (Class|PlayerController|SetMouseCursorWidget _returnvalue_2 "Crosshairs")
        (Transformation|SetWorldLocation (Variables|Default|GetMainPen) (Math|Vector|MakeVector _x 1.4e+02 _z) true false)))))

(event EventBeginPlay
  ;[1 1 1] Begin Play Enable Input
  (Input|EnableInput (Game|GetPlayerController 0)))

(event Input|MouseEvents|LeftMouseButton
  (params (Key :type Key%20Structure))
  ;[1 1 1] Change Camera To WhiteBoard
  ;;[1 1 1] Set Left Mouse button Held Variable
  (:Pressed
    (Variables|Default|Setlmbheld true))
  (:Released
    (Variables|Default|Setlmbheld false)))

(event Input|KeyboardEvents|F
  (params (Key :type Key%20Structure))
  (bind _returnvalue (Game|GetPlayerController 0))
  ;[1 1 1] Change Camera To WhiteBoard
  (:Pressed
    (Utilities|FlowControl|FlipFlop
      (:A
        (Game|Player|SetViewTargetwithBlend _returnvalue self 1.0 "VTBlend_Linear" 0.0 false)
        (Variables|/Script/Engine.PlayerController|SetbShowMouseCursor _returnvalue true)
        (Variables|Default|SetUsingWhiteBoard true))
      (:B
        (Game|Player|SetViewTargetwithBlend _returnvalue (Game|Player|GetPlayerPawn 0) 1.0 "VTBlend_Linear" 0.0 false)
        (Variables|/Script/Engine.PlayerController|SetbShowMouseCursor _returnvalue false)
        (Variables|Default|SetUsingWhiteBoard false)))))

(fn ConstructionScript
  (Rendering|Material|SetMaterial (Variables|Default|GetMainPen) 0 "/Game/pencil_lambert1_BaseColor_Mat.pencil_lambert1_BaseColor_Mat"))